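; AI controller that runs the BT_AI behavior tree and tracks a target through AI perception.
; Perception updates go to SightDetection, which writes the sensed actor to the TargetActor blackboard key, or clears it on lost sight or any non-sight stimulus.
; When the controller is a BP_AI_Controller_Boss, detection also activates or deactivates boss combat.
; DamageDetection is an uncalled stub that only checks the sense class.
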(event OnTargetPerceptionUpdated(AIPerception)
  (params (Actor :type Actor%20Object%20Reference) (Stimulus :type AI%20Stimulus%20Structure))
  ;[1 1 1] Detect & Chase Actors
  (CallFunction|SightDetection Actor Stimulus))

(event EventBeginPlay
  (AI|RunBehaviorTree "/Game/AI/BT_AI.BT_AI"))

(fn ConstructionScript)

(fn SightDetection
  (params (Actor :type Actor%20Object%20Reference) (Stimulus :type AI%20Stimulus%20Structure))
  (bind _returnvalue (Class|AIPerceptionSystem|GetSenseClassforStimulus Stimulus))
  (if (== _returnvalue "/Script/AIModule.AISense_Sight")
    (if (.bSuccessfullySensed (Utilities|Struct|BreakAIStimulus Stimulus))
      (AI|Components|Blackboard|SetValueasObject (AI|GetBlackboard 0) (Utilities|Name|MakeLiteralName "TargetActor") Actor)
      (bind _asbp_ai_controller_boss (Utilities|Casting|CastToBP_AI_Controller_Boss self))
      (Default|ActivateBossCombat _asbp_ai_controller_boss)
      (else
        (AI|Components|Blackboard|SetValueasObject (AI|GetBlackboard 0) (Utilities|Name|MakeLiteralName "TargetActor") 0 :!label _label)
        (bind _asbp_ai_controller_boss_2 (Utilities|Casting|CastToBP_AI_Controller_Boss self))
        (Default|DeactivateBossCombat _asbp_ai_controller_boss_2)))
    (else
      (goto _label))))

(fn DamageDetection
  (params (Actor :type Actor%20Object%20Reference) (Stimulus :type AI%20Stimulus%20Structure))
  (bind _returnvalue (Class|AIPerceptionSystem|GetSenseClassforStimulus Stimulus))
  (if (== _returnvalue "/Script/AIModule.AISense_Damage")
    _))