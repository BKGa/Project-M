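; BP_AI_Boss is the boss AI character Blueprint.
; Each tick it casts its AI controller to BP_AI_Controller_Boss and copies current and max health from its player stats component into that controller.
; The same tick sets its base damage to a fixed value, and the construction script only calls the parent.
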(event EventBeginPlay
  (|CallParentFunction) ; This node is disabled and will not be called.\nDrag off pins to build functionality.
)

(event Collision|EventActorBeginOverlap
  (params (OtherActor :type Actor%20Object%20Reference))
  (|CallParentFunction OtherActor) ; This node is disabled and will not be called.\nDrag off pins to build functionality.
)

(event EventTick
  (params (DeltaSeconds :type Float%20%28single-precision%29))
  (bind _bpc_player_stats (Variables|Default|GetBPC_Player_Stats))
  (|CallParentFunction DeltaSeconds)
  (bind _asbp_ai_controller_boss (Utilities|Casting|CastToBP_AI_Controller_Boss (AI|GetAIController self)))
  (Variables|/Game/AI/Boss_AI/BP_AI_Controller_Boss.BP_AI_Controller_Boss_C|SetBoss%20Health _asbp_ai_controller_boss (Variables|/Game/ThirdPerson/Blueprints/BPC_Player_Stats.BPC_Player_Stats_C|GetCurrent%20Health _bpc_player_stats))
  (Variables|/Game/AI/Boss_AI/BP_AI_Controller_Boss.BP_AI_Controller_Boss_C|SetBoss%20Max%20Health _asbp_ai_controller_boss (Variables|/Game/ThirdPerson/Blueprints/BPC_Player_Stats.BPC_Player_Stats_C|GetMax%20Health _bpc_player_stats))
  (Variables|Default|SetBase%20Damage 5e+01))

(fn ConstructionScript
  (|CallParentFunction))