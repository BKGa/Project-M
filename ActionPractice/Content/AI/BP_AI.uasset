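; Enemy AI character that fights with a sword combo, requested through Attack or a behavior-tree call.
; AttackIndex and GonnaCombo chain the attack montages, while a looping timer sphere-traces the blade to damage "Damageable" actors with blood and sound.
; Taking damage breaks the combo, plays a random hit montage, launches it along the player's facing and lowers BPCPlayerStats health.
; Tick turns the health bar toward the camera and handles zero-health ragdoll, explosion and destruction.
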(event Custom|Sword%20Attack
  ;[1 1 1] Combo System
  ;;[1 1 1] Sword Attack
  (Utilities|FlowControl|Delay 0.1)
  (if (Variables|Default|GetAttacking?)
    (Variables|Default|SetGonna%20Combo? true)
    (else
      (Variables|Default|SetAttacking? true)
      (switch int (Variables|Default|GetAttack%20index)
        (:0
          (CallFunction|SwordAttack1))
        (:1
          (CallFunction|SwordAttack2))
        (:2
          (CallFunction|SwordAttack4))))))

(event Custom|Sword%20Attack%20Combo
  ;[1 1 1] Combo System
  ;;[1 1 1] Sword Combo
  (if (Variables|Default|GetGonna%20Combo?)
    (Variables|Default|SetGonna%20Combo? false)
    (switch int (Variables|Default|GetAttack%20index)
      (:0
        (CallFunction|SwordAttack1))
      (:1
        (CallFunction|SwordAttack2))
      (:2
        (CallFunction|SwordAttack4)))
    (else
      (CallFunction|StopCombo))))

(event Custom|Play%20Sword%20Hit%20Sounds
  (Audio|PlaySoundatLocation "/Game/Audio/Attacks/536105__eminyildirim__sword-hit-medium.536105__eminyildirim__sword-hit-medium" (Transformation|GetActorLocation (Components|GetOwner)) "0, 0, 0" 1.0 1.0 0.0 0 0 0 0))

(event Custom|Sword%20Attack%20Combo%20Call%20from%20BT
  ;[1 1 1] Combo System
  (if (Variables|Default|GetAble%20to%20Attack?)
    (CallFunction|SwordAttack)))

(event Custom|Stop%20Combo
  ;[1 1 1] Combo System
  ;;[1 1 1] Stop Combo
  (Variables|Default|SetAttacking? false)
  (Variables|Default|SetAttack%20index 0))

(event Custom|Sword%20Attack%204
  ;[1 1 1] Combo System
  ;;[1 1 1] Sword Attack 4
  (Utilities|FlowControl|DoOnce false
    (:Completed
      (Utilities|FlowControl|Delay 0.1)
      (Animation|Montage|PlayMontage (Variables|Character|GetMesh) "/Game/Characters/Player/Animation/Attacks/Attack3_Montage.Attack3_Montage" (Variables|Default|GetSword%20Attack%20Animation%20Speed)
        (:then
          (Variables|Default|SetAttack%20index 4))))))

(event Custom|Sword%20Attack%201
  ;[1 1 1] Combo System
  ;;[1 1 1] Sword Attack 1
  (Utilities|FlowControl|DoOnce false :!label _label
    (:Completed
      (Utilities|FlowControl|Delay 0.1)
      (Animation|Montage|PlayMontage (Variables|Character|GetMesh) "/Game/Characters/Player/Animation/Attacks/Attack1_Montage.Attack1_Montage" (Variables|Default|GetSword%20Attack%20Animation%20Speed)
        (:then
          (Variables|Default|SetAttack%20index 1)
          (goto _label Reset))))))

(event Custom|Sword%20Trace%20Loop
  ;[1 1 1] Sword Tracer
  (bind (_outhit _returnvalue) (Collision|SphereTraceByChannel (Transformation|GetWorldLocation (Variables|Default|GetSword%20Top%20Point)) (Transformation|GetWorldLocation (Variables|Default|GetSword%20Bottom%20Point)) 12.0 "TraceTypeQuery1" false 0 "None" true "(R=1.000000,G=0.000000,B=0.000000,A=1.000000)" "(R=0.000000,G=1.000000,B=0.000000,A=1.000000)" 0.2))
  (if _returnvalue
    (if (Actor|ActorHasTag (.HitActor (Collision|BreakHitResult _outhit)) "Damageable")
      (Utilities|FlowControl|DoOnce false :!label _label
        (:Completed
          (Game|Damage|ApplyDamage (.HitActor (Collision|BreakHitResult _outhit)) (Variables|Default|GetBase%20Damage) 0 0)
          (CallFunction|PlaySwordHitSounds)
          (Effects|SpawnEmitteratLocation "/Game/Realistic_Starter_VFX_Pack_Vol2/Particles/Blood/P_Blood_Splat_Cone.P_Blood_Splat_Cone" (.Location (Collision|BreakHitResult _outhit)) (Math|Rotator|MakeRotfromXY (.Normal (Collision|BreakHitResult _outhit)) (.Normal (Collision|BreakHitResult _outhit))))
          (Utilities|FlowControl|Delay 0.5)
          (goto _label Reset))))))

(event Custom|Sword%20Attack%202
  ;[1 1 1] Combo System
  ;;[1 1 1] Sword Attack 2
  (Utilities|FlowControl|DoOnce false :!label _label
    (:Completed
      (Utilities|FlowControl|Delay 0.1)
      (Animation|Montage|PlayMontage (Variables|Character|GetMesh) "/Game/Characters/Player/Animation/Attacks/Attack2_Montage.Attack2_Montage" (Variables|Default|GetSword%20Attack%20Animation%20Speed)
        (:then
          (Variables|Default|SetAttack%20index 2)
          (goto _label Reset))))))

(event Custom|Start%20Sword%20Trace
  ;[1 1 1] Sword Tracer
  (bind _returnvalue (Utilities|Time|SetTimerbyEvent (delegate Custom|Sword%20Trace%20Loop) 0.001 true))
  (Variables|Default|SetSwordTraceLoop _returnvalue))

(event Custom|Sword%20Attack%203
  ;[1 1 1] Combo System
  ;;[1 1 1] Sword Attack 3 (Unused)
  (Utilities|FlowControl|DoOnce false :!label _label
    (:Completed
      (Utilities|FlowControl|Delay 0.1)
      (Animation|Montage|PlayMontage (Variables|Character|GetMesh) "/Game/Characters/Player/Animation/Attacks/Kick_Montage.Kick_Montage" (Variables|Default|GetSword%20Attack%20Animation%20Speed)
        (:then
          (Variables|Default|SetAttack%20index 3)
          (goto _label Reset))))))

(event Custom|Stop%20Sword%20Trace
  ;[1 1 1] Sword Tracer
  (Utilities|Time|ClearandInvalidateTimerbyHandle (Variables|Default|GetSwordTraceLoop)))

(event EventBeginPlay
  (bind _aswb_dummy_health_bar (Utilities|Casting|CastToWB_Dummy_Health_Bar (UserInterface|GetWidget (Variables|Default|GetHealth%20Bar%20Widget))))
  (Variables|Default|SetHealthBarUI _aswb_dummy_health_bar))

(event Collision|EventActorBeginOverlap
  (params (OtherActor :type Actor%20Object%20Reference)))

(event Game|Damage|EventAnyDamage
  (params (Damage :type Float%20%28single-precision%29) (DamageType :type Damage%20Type%20Object%20Reference) (InstigatedBy :type Controller%20Object%20Reference) (DamageCauser :type Actor%20Object%20Reference))
  (CallFunction|StopCombo)
  (Development|PrintString "I HAVE BEEN DAMAGED! OW!")
  (Animation|PlayAnimMontage (Utilities|Array|Get(acopy) (Variables|Default|GethitAnims) (Math|Random|RandomIntegerinRange 0 (- (Utilities|Array|Length (Variables|Default|GethitAnims)) 1))) 1.0 "None")
  (bind _asbp_third_person_character (Utilities|Casting|CastToBP_ThirdPersonCharacter (Game|GetPlayerCharacter 0)))
  (Character|LaunchCharacter (* (Math|Vector|GetForwardVector (Transformation|GetActorRotation _asbp_third_person_character)) 1e+03) false false)
  (Default|DecreaseHealth (Variables|Default|GetBPC_Player_Stats) Damage)
  (Collision|SetCollisionObjectType (Variables|Character|GetMesh) "ECC_PhysicsBody"))

(event EventTick
  (params (DeltaSeconds :type Float%20%28single-precision%29))
  (bind _health_bar_widget (Variables|Default|GetHealth%20Bar%20Widget))
  (bind _mesh (Variables|Character|GetMesh))
  (bind _returnvalue (Components|GetOwner _mesh))
  (bind _returnvalue_2 (Transformation|GetActorLocation _returnvalue))
  (Transformation|SetWorldRotation _health_bar_widget (Math|Rotator|FindLookatRotation (Transformation|GetWorldLocation _health_bar_widget) (Transformation|GetWorldLocation (Variables|/Script/Engine.PlayerCameraManager|GetTransformComponent (Game|GetPlayerCameraManager 0)))) false false)
  (if (== (Variables|/Game/ThirdPerson/Blueprints/BPC_Player_Stats.BPC_Player_Stats_C|GetCurrent%20Health (Variables|Default|GetBPC_Player_Stats)) 0.0)
    (Rendering|SetVisibility (Variables|Default|GetHealth%20Bar%20Widget) false false)
    (Utilities|FlowControl|Delay 0.1)
    (Physics|SetSimulatePhysics (Variables|Character|GetMesh) true)
    (Utilities|FlowControl|Delay 0.2)
    (Utilities|FlowControl|DoOnce false
      (:Completed
        (Utilities|FlowControl|Delay 1.0)
        (Physics|AddImpulse (Variables|Character|GetMesh) "100.000000,100.000000,100000.000000" "None" false)
        (Effects|SpawnEmitteratLocation "/Game/StarterContent/Particles/P_Explosion.P_Explosion" _returnvalue_2 "0, 0, 0" "2.000000,2.000000,2.000000")
        (Audio|PlaySoundatLocation "/Game/StarterContent/Audio/Explosion01.Explosion01" _returnvalue_2 "0, 0, 0" 1.0 1.0 0.0 0 0 0 0)
        (Actor|DestroyActor)))))

(fn ConstructionScript)

(fn Attack
  (CallFunction|SwordAttackComboCallfromBT)
  (return 0.0))