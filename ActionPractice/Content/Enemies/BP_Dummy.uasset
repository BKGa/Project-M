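; BP_Dummy is a damageable enemy dummy Character with a floating health bar and an explosive death.
; Any damage plays a random hit montage, launches it along the player's facing direction and lowers health in BPCPlayerStats.
; Tick turns the health bar toward the camera and polls for zero health.
; At zero it hides the bar, ragdolls, then after delays gets an impulse, explodes with effects and sound, and destroys itself.
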(event Custom|Ragdoll
  (Utilities|FlowControl|Delay 0.1)
  (Physics|SetSimulatePhysics (Variables|Character|GetMesh) true))

(event EventBeginPlay
  (bind _aswb_dummy_health_bar (Utilities|Casting|CastToWB_Dummy_Health_Bar (UserInterface|GetWidget (Variables|Default|GetHealth%20Bar%20Widget))))
  (Variables|Default|SetHealthBarUI _aswb_dummy_health_bar))

(event Collision|EventActorBeginOverlap
  (params (OtherActor :type Actor%20Object%20Reference)))

(event Game|Damage|EventAnyDamage
  (params (Damage :type Float%20%28single-precision%29) (DamageType :type Damage%20Type%20Object%20Reference) (InstigatedBy :type Controller%20Object%20Reference) (DamageCauser :type Actor%20Object%20Reference))
  (Development|PrintString "I HAVE BEEN DAMAGED! OW!")
  (Animation|PlayAnimMontage (Utilities|Array|Get(acopy) (Variables|Default|GethitAnims) (Math|Random|RandomIntegerinRange 0 (- (Utilities|Array|Length (Variables|Default|GethitAnims)) 1))) 1.0 "None")
  (bind _asbp_third_person_character (Utilities|Casting|CastToBP_ThirdPersonCharacter (Game|GetPlayerCharacter 0)))
  (Character|LaunchCharacter (* (Math|Vector|GetForwardVector (Transformation|GetActorRotation _asbp_third_person_character)) 1e+03) false false)
  (Default|DecreaseHealth (Variables|Default|GetBPC_Player_Stats) Damage))

(event EventTick
  (params (DeltaSeconds :type Float%20%28single-precision%29))
  (bind _mesh (Variables|Character|GetMesh))
  (bind _health_bar_widget (Variables|Default|GetHealth%20Bar%20Widget))
  (bind _returnvalue (Components|GetOwner _mesh))
  (bind _returnvalue_2 (Transformation|GetActorLocation _returnvalue))
  (Transformation|SetWorldRotation _health_bar_widget (Math|Rotator|FindLookatRotation (Transformation|GetWorldLocation _health_bar_widget) (Transformation|GetWorldLocation (Variables|/Script/Engine.PlayerCameraManager|GetTransformComponent (Game|GetPlayerCameraManager 0)))) false false)
  (if (== (Variables|/Game/ThirdPerson/Blueprints/BPC_Player_Stats.BPC_Player_Stats_C|GetCurrent%20Health (Variables|Default|GetBPC_Player_Stats)) 0.0)
    (Rendering|SetVisibility (Variables|Default|GetHealth%20Bar%20Widget) false false)
    (CallFunction|Ragdoll)
    (Utilities|FlowControl|Delay 0.2)
    (Utilities|FlowControl|DoOnce false
      (:Completed
        (Utilities|FlowControl|Delay 1.0)
        (Physics|AddImpulse (Variables|Character|GetMesh) "100.000000,100.000000,100000.000000" "None" false)
        (Effects|SpawnEmitteratLocation "/Game/StarterContent/Particles/P_Explosion.P_Explosion" _returnvalue_2 "0, 0, 0" "2.000000,2.000000,2.000000")
        (Audio|PlaySoundatLocation "/Game/StarterContent/Audio/Explosion01.Explosion01" _returnvalue_2 "0, 0, 0" 1.0 1.0 0.0 0 0 0 0)
        (Actor|DestroyActor)))))

(fn ConstructionScript)